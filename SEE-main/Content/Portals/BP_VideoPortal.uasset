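; BP_VideoPortal is a portal trigger that plays a fullscreen video widget when the player pawn overlaps its Box.
; On overlap it stores TeleTag in GI_Main's TeportTag, then creates a WP_MediaPlayer widget with its media player and playlist.
; The media player's end-reached event removes the widget from the viewport.
; An OpenLevelByName node is left unconnected, so the portal itself does not change level.
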(event OnComponentBeginOverlap(Box)
  (params (OverlappedComponent :type Primitive%20Component%20Object%20Reference) (OtherActor :type Actor%20Object%20Reference) (OtherComp :type Primitive%20Component%20Object%20Reference) (OtherBodyIndex :type Integer) (bFromSweep :type Boolean) (SweepResult :type Hit%20Result%20Structure%20%28by%20ref%29))
  (bind _mediaplayer (Variables|Default|GetMediaPlayer))
  (if (== OtherActor (Game|Player|GetPlayerPawn 0))
    (bind _asgi_main (Utilities|Casting|CastToGI_Main (Game|GetGameInstance)))
    (Variables|/Game/GI_Main.GI_Main_C|SetTeportTag _asgi_main (Variables|Default|GetTeleTag))
    (bind _returnvalue (UserInterface|CreateWidget "/Game/Sreen/WP_MediaPlayer.WP_MediaPlayer_C" 0 _mediaplayer "/Game/Sreen/Freddy_Fazbear_x_Whistle__Josh_Hutcherson_.Freddy_Fazbear_x_Whistle__Josh_Hutcherson_"))
    (UserInterface|Viewport|AddtoViewport _returnvalue 0)
    (Media|MediaPlayer|BindEventtoOnEndReached _mediaplayer (delegate Custom|VideoEnd))))

(event Custom|VideoEnd
  (Widget|RemovefromParent (stale OnComponentBeginOverlap(Box) _returnvalue)))

(event EventBeginPlay)

(event EventTick
  (params (DeltaSeconds :type Float%20%28single-precision%29)))

(fn ConstructionScript)