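; BP_MonsterPawn is a monster NPC that chases the player and is meant to load LEVEL3 on contact.
; BeginPlay calls Roam, which despite its name issues a single AI MoveTo toward the BP_TOPDOWN player character.
; The BoxCollision hit event compares HitComponent, its own component, to the player character instead of OtherActor, so the level load cannot fire as written.
; A walk speed setter is left unconnected.
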(event OnComponentHit(BoxCollision)
  (params (HitComponent :type Primitive%20Component%20Object%20Reference) (OtherActor :type Actor%20Object%20Reference) (OtherComp :type Primitive%20Component%20Object%20Reference) (NormalImpulse :type Vector :default "0, 0, 0") (Hit :type Hit%20Result%20Structure%20%28by%20ref%29))
  (if (== HitComponent (Game|GetPlayerCharacter 0))
    (Game|OpenLevel(byName) "LEVEL3")))

(event Custom|Roam
  (bind _asbp_topdown (Utilities|Casting|CastToBP_TOPDOWN (Game|GetPlayerCharacter 0)))
  (AI|AIMoveTo self "0, 0, 0" _asbp_topdown 2e+02 false))

(event Collision|EventActorBeginOverlap
  (params (OtherActor :type Actor%20Object%20Reference)))

(event EventTick
  (params (DeltaSeconds :type Float%20%28single-precision%29)))

(event EventBeginPlay
  (CallFunction|Roam))

(fn ConstructionScript)