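; BP_Monster is a monster NPC that chases the player and triggers a level change on contact.
; On BeginPlay it calls Roam, which issues a single AIMoveTo toward the BP_TOPDOWN player, and sets its walk speed.
; Player overlap with BoxCollison clears all widgets and opens SCREAM, while a capsule hit opens LEVEL3.
; An unconnected chain that would show a screamer video widget before opening LEVEL3 never runs.
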(event OnComponentHit(CapsuleComponent)
  (params (HitComponent :type Primitive%20Component%20Object%20Reference) (OtherActor :type Actor%20Object%20Reference) (OtherComp :type Primitive%20Component%20Object%20Reference) (NormalImpulse :type Vector :default "0, 0, 0") (Hit :type Hit%20Result%20Structure%20%28by%20ref%29))
  (if (== OtherActor (Game|GetPlayerCharacter 0))
    (Game|OpenLevel(byName) "LEVEL3")))

(event OnComponentBeginOverlap(BoxCollison)
  (params (OverlappedComponent :type Primitive%20Component%20Object%20Reference) (OtherActor :type Actor%20Object%20Reference) (OtherComp :type Primitive%20Component%20Object%20Reference) (OtherBodyIndex :type Integer) (bFromSweep :type Boolean) (SweepResult :type Hit%20Result%20Structure%20%28by%20ref%29))
  (if (== OtherActor (Game|GetPlayerCharacter 0))
    (Viewport|RemoveAllWidgets)
    (Game|OpenLevel(byName) "SCREAM")))

(event Custom|Roam
  (bind _asbp_topdown (Utilities|Casting|CastToBP_TOPDOWN (Game|GetPlayerCharacter 0)))
  (AI|AIMoveTo self "0, 0, 0" _asbp_topdown 2e+02 false))

(event Collision|EventActorBeginOverlap
  (params (OtherActor :type Actor%20Object%20Reference)))

(event EventTick
  (params (DeltaSeconds :type Float%20%28single-precision%29)))

(event EventBeginPlay
  (CallFunction|Roam)
  (Variables|/Script/Engine.CharacterMovementComponent|SetMaxWalkSpeed (Variables|Character|GetCharacterMovement) 5.5e+02))

(fn ConstructionScript)