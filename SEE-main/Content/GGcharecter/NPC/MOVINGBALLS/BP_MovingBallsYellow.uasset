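; BP_MovingBallsYellow is a wandering NPC ball that the player collects by running into it.
; It roams by AI MoveTo to random reachable points nearby, restarting after a short delay on each success.
; A capsule hit from the player increments the Balls counter on the cached BP_TOPDOWN and destroys the ball.
; When the count reaches twelve, it moves the BP_portal at index 1 to a fixed location.
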(event OnComponentHit(CapsuleComponent)
  (params (HitComponent :type Primitive%20Component%20Object%20Reference) (OtherActor :type Actor%20Object%20Reference) (OtherComp :type Primitive%20Component%20Object%20Reference) (NormalImpulse :type Vector :default "0, 0, 0") (Hit :type Hit%20Result%20Structure%20%28by%20ref%29))
  (bind _charcount (Variables|Default|GetCharCount))
  (if (== OtherActor (Game|GetPlayerCharacter 0))
    (Variables|/Game/GGcharecter/BP_TOPDOWN.BP_TOPDOWN_C|SetBalls _charcount (+ (Variables|/Game/GGcharecter/BP_TOPDOWN.BP_TOPDOWN_C|GetBalls _charcount) 1))
    (Actor|DestroyActor)
    (if (== (Variables|/Game/GGcharecter/BP_TOPDOWN.BP_TOPDOWN_C|GetBalls _charcount) 12)
      (bind _outactors (Actor|GetAllActorsOfClass "/Game/Portals/BP_portal.BP_portal_C"))
      (Transformation|SetActorLocation (Utilities|Array|Get(acopy) _outactors 1) "-4711.253167,-2648.050461,936.378303" false false))))

(event Custom|Roaming
  (AI|AIMoveTo self (.RandomLocation (AI|Navigation|GetRandomReachablePointinRadius (Transformation|GetWorldLocation (Variables|Character|GetMesh)) 5e+02 0 0)) 0 5.0 false
    (:OnSuccess
      (Utilities|FlowControl|Delay 0.1)
      (CallFunction|Roaming))))

(event Custom|CharRef
  (bind _outactors (Actor|GetAllActorsOfClass "/Game/GGcharecter/BP_TOPDOWN.BP_TOPDOWN_C"))
  (Variables|Default|SetCharCount (Utilities|Array|Get(acopy) _outactors)))

(event EventBeginPlay
  (CallFunction|Roaming)
  (CallFunction|CharRef))

(fn ConstructionScript)