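; GM_BASE is a base game mode that handles player spawn placement and starts dialogue.
; ChoosePlayerStart picks the PlayerStart whose tag matches the TeportTag held in GI_Main, so the game instance determines the spawn point.
; StartDialogue opens a DemoDialogueWidget with the given dialogue, disables input on the BP_TOPDOWN player character and shows the mouse cursor.
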(event EventBeginPlay)

(event EventTick
  (params (DeltaSeconds :type Float%20%28single-precision%29)))

(fn ConstructionScript)

(fn ChoosePlayerStart
  (params (Player :type Controller%20Object%20Reference))
  (bind _asgi_main (Utilities|Casting|CastToGI_Main (Game|GetGameInstance)))
  (bind _outactors (Actor|GetAllActorsOfClass "/Script/Engine.PlayerStart"))
  (for _array_element _outactors
    (if (== (Variables|/Script/Engine.PlayerStart|GetPlayerStartTag _array_element) (Variables|/Game/GI_Main.GI_Main_C|GetTeportTag _asgi_main))
      (return _array_element))))

(fn StartDialogue
  (params (Dialogue :type Dialogue%20Object%20Reference))
  (bind _asbp_topdown (Utilities|Casting|CastToBP_TOPDOWN (Game|GetPlayerCharacter 0)))
  (bind _returnvalue (UserInterface|CreateWidget "/DialoguePlugin/UI/DemoDialogueWidget.DemoDialogueWidget_C" 0 Dialogue 0))
  (UserInterface|Viewport|AddtoViewport _returnvalue 0)
  (Input|DisableInput _asbp_topdown 0)
  (Variables|/Script/Engine.PlayerController|SetbShowMouseCursor (Game|GetPlayerController 0) true))